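; BP_FlamePillar is a flame pillar actor that gives its fire light a continuous, varying flicker.
; On BeginPlay it randomly plays one of two intensity timelines, then picks again each time one finishes, so the pattern loops with variation.
; Each timeline update feeds its curve value to ScaleFlameIntensity, which multiplies it by BaseIntensity and sets the FireLight intensity.
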(event Custom|StartTimeline
  (bind _flameintensity (Timeline|FlameIntensity PlayFromStart)
    (:Update
      (CallFunction|ScaleFlameIntensity _flameintensity))
    (:Finished
      (CallFunction|ChooseTimeline))))

(event Custom|StartTimeline_Alt
  (bind _flameintensity_alternative (Timeline|FlameIntensity_2 PlayFromStart)
    (:Update
      (CallFunction|ScaleFlameIntensity _flameintensity_alternative))
    (:Finished
      (CallFunction|ChooseTimeline))))

(event Custom|ChooseTimeline
  (switch int (Math|Random|RandomIntegerinRange 0 1)
    (:0
      (CallFunction|StartTimeline))
    (:1
      (CallFunction|StartTimelineAlt))))

(event EventBeginPlay
  (CallFunction|ChooseTimeline))

(fn ConstructionScript)

(fn ScaleFlameIntensity
  (params (Intensity :type Float%20%28double-precision%29))
  (Rendering|Components|Light|SetIntensity (Variables|Default|GetFireLight) (* Intensity (Variables|Default|GetBaseIntensity))))