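; Aura's Electrocute lightning ability, a channeled beam aimed at the mouse hit and held until input release.
; Activation turns the avatar to the target, plays a montage, and on its event locks movement and spawns the beam.
; The beam is a ShockLoop gameplay cue, placed on the traced target if it implements CombatInterface, otherwise on the avatar.
; Release removes the cue, restores cursor and walking, then ends the ability.
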(event Ability|EventActivateAbility
  (bind _ownercharacter (Variables|Default|GetOwnerCharacter))
  (bind _charactermovement (Variables|/Script/Engine.Character|GetCharacterMovement _ownercharacter))
  (CallFunction|EnforceCombatInterface)
  ;[1 0.6832 0.9138] Store Mouse Data Variables
  (bind _datahandle (|TargetDataUnderMouse)
    (:ValidData
      (Class|AuraBeamSpell|StoreMouseDataInfo (Ability|TargetData|GetHitResultfromTargetData _datahandle))
      (Class|AuraBeamSpell|StoreOwnerParams)
      (Utilities|FlowControl|Sequence
        (:then_0
          (Variables|/Script/Engine.PlayerController|SetbShowMouseCursor (Variables|Default|GetOwnerPlayerController) false)
          (Class|CombatInterface|UpdateFacingTarget(Message) (Ability|GetAvatarActorfromActorInfo) (Variables|Default|GetMouseHitLocation))
          (GameplayCue|ExecuteGameplayCue :GameplayCueTag "(TagName=\"GameplayCue.ShockBurst\")")
          (|PlayMontageandWaitProxy "None" (Variables|Default|GetMontage%20Electrocute) 1.0 "None" false 1.0 0.0 false
            (:then
              (Ability|Tasks|WaitGameplayEvent "(TagName=\"Event.Montage.Electrocute\")" 0
                (:EventReceived
                  (Class|CombatInterface|SetinShockLoop(Message) (Ability|GetAvatarActorfromActorInfo) true)
                  (Pawn|Components|CharacterMovement|DisableMovement _charactermovement)
                  (CallFunction|SpawnElectricBeam))))))
        (:then_1
          (Ability|Tasks|WaitInputRelease false
            (:OnRelease
              (Variables|/Script/Engine.PlayerController|SetbShowMouseCursor (Variables|Default|GetOwnerPlayerController) true)
              (Class|CombatInterface|SetinShockLoop(Message) (Ability|GetAvatarActorfromActorInfo) false)
              (if (Variables|Default|GetFirstTargetIsInterface)
                (GameplayCue|RemoveGameplayCueOnActor(Looping) (Variables|Default|GetTargetActor) "(TagName=\"GameplayCue.ShockLoop\")" (Variables|Default|GetFirstTargetCueParams))
                (else
                  (GameplayCue|RemoveGameplayCueOnActor(Looping) (Ability|GetAvatarActorfromActorInfo) "(TagName=\"GameplayCue.ShockLoop\")" (Variables|Default|GetFirstTargetCueParams))))
              (Pawn|Components|CharacterMovement|SetMovementMode _charactermovement "MOVE_Walking" 0)
              (Ability|EndAbility))))))))

(fn EnforceCombatInterface
  (if (not (Utilities|DoesObjectImplementInterface (Ability|GetAvatarActorfromActorInfo) "/Script/Aura.CombatInterface"))
    (Ability|EndAbility)))

(fn SpawnElectricBeam
  (Class|AuraBeamSpell|TraceFrontmostTarget (Variables|Default|GetMouseHitLocation))
  (bind _returnvalue (Class|CombatInterface|GetWeapon(Message) (Variables|Default|GetOwnerCharacter)))
  (Variables|Default|SetFirstTargetCueParams (Ability|GameplayCue|MakeGameplayCueParameters :Location (Variables|Default|GetMouseHitLocation) :SourceObject (Variables|Default|GetTargetActor) :TargetAttachComponent _returnvalue))
  ;[1 1 1] Is Target Actor (MouseHit) an enemy?
  (bind _output_get (Variables|Default|SetFirstTargetIsInterface (Utilities|DoesObjectImplementInterface (Variables|Default|GetTargetActor) "/Script/Aura.CombatInterface")))
  (if _output_get
    (LocalVariables|SetCueTarget (Variables|Default|GetTargetActor))
    (else
      (LocalVariables|SetCueTarget (Ability|GetAvatarActorfromActorInfo))))
  (GameplayCue|AddGameplayCueOnActor(Looping) (LocalVariables|GetCueTarget) "(TagName=\"GameplayCue.ShockLoop\")" (Variables|Default|GetFirstTargetCueParams)))